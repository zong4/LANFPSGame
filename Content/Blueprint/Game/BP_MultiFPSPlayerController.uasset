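; Player controller for multiplayer FPS deathmatch, linking each player to DeathMatchGameMode and their HUD.
; On death it reports the death and instigating killer to the game mode, destroys the pawn and requests a respawn, then possesses the character it spawns.
; It creates the local W_PlayerUI and forwards health, ammo, crosshair recoil and sorted scoreboard values to it.
; Client events handle input, cursor, match time and return to main menu.
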(event Custom|SpawnPlayerCharacter
  (params (Class :type FPS%20Teach%20Base%20Character%20Class%20Reference) (SpawnTransform :type Transform))
  (bind _returnvalue (Game|SpawnActorfromClass Class SpawnTransform "Undefined" 0 0))
  (Pawn|Possess _returnvalue)
  (CallFunction|ClientHideMouse))

(event Custom|StartSpawnCharacter
  (Utilities|FlowControl|Delay 1.0)
  (bind _asdeath_match_game_mode (Utilities|Casting|CastToDeathMatchGameMode (Game|GetGameMode)))
  (Default|RequstSpawn _asdeath_match_game_mode self))

(event Custom|UpdateValues
  (params (Values :type Array%20of%20Death%20Match%20Player%20Data%20Structures))
  (bind _output_get (Variables|Default|SetValues Values))
  (Class|KismetMultiFPSLibrary|SortValues _output_get)
  (bind _playerui (Variables|Default|GetPlayerUI)
    (:then
      (Default|UpdateSortBox _playerui (Variables|Default|GetValues)))
    (:else)))

(event Custom|ServerRequireUpdateValues
  (bind _asdeath_match_game_mode (Utilities|Casting|CastToDeathMatchGameMode (Game|GetGameMode)))
  (Default|UpdateValues _asdeath_match_game_mode))

(event Custom|ClientDisableInput
  (Input|DisableInput (Pawn|GetControlledPawn) self))

(event Custom|ClientUpdateDownTime
  (params (DownTime :type Integer))
  (Variables|Default|SetDownTime DownTime))

(event Custom|ClientEndGame
  (Game|OpenLevel(byName) "MainMenu"))

(event Custom|ClientHideMouse
  (Input|SetInputModeGameOnly self)
  (Variables|Default|SetbShowMouseCursor false))

(event EventDoCrosshairRecoil
  ;[1 1 1] UI
  (Default|DoCrosshairRecoil (Variables|Default|GetPlayerUI)))

(event EventUpdateAmmoUI
  (params (ClipCurrentAmmo :type Integer) (GunCurrentAmmo :type Integer))
  ;[1 1 1] UI
  (Default|UpdateAmmo (Variables|Default|GetPlayerUI) ClipCurrentAmmo GunCurrentAmmo))

(event EventCreatePlayerUI
  ;[1 1 1] UI
  (Variables|Default|GetPlayerUI
    (:then
      (Widget|RemovefromParent (Variables|Default|GetPlayerUI))
      (if (Pawn|IsLocalPlayerController)
        (bind _returnvalue (UserInterface|CreateWidget "/Game/Blueprint/GameUI/W_PlayerUI.W_PlayerUI_C" self))
        (bind _output_get (Variables|Default|SetPlayerUI _returnvalue))
        (UserInterface|Viewport|AddtoViewport _output_get 0)
        (CallFunction|ServerRequireUpdateValues)))
    (:else
      (if (Pawn|IsLocalPlayerController)
        (bind _returnvalue_2 (UserInterface|CreateWidget "/Game/Blueprint/GameUI/W_PlayerUI.W_PlayerUI_C" self))
        (bind _output_get_2 (Variables|Default|SetPlayerUI _returnvalue_2))
        (UserInterface|Viewport|AddtoViewport _output_get_2 0)
        (CallFunction|ServerRequireUpdateValues)))))

(event EventUpdateHealthUI
  (params (NewHealth :type Float%20%28single-precision%29))
  ;[1 1 1] UI
  (Default|UpdateHealth (Variables|Default|GetPlayerUI) NewHealth))

(event EventDeathMatchDeath
  (params (DamageCauser :type Actor%20Object%20Reference))
  (bind _asdeath_match_game_mode (Utilities|Casting|CastToDeathMatchGameMode (Game|GetGameMode)))
  (Default|SelfDeath _asdeath_match_game_mode self)
  (CallFunction|ClientDisableInput)
  (bind _asbp_multi_fpsplayer_controller (Utilities|Casting|CastToBP_MultiFPSPlayerController (Game|GetInstigatorController DamageCauser)))
  (Default|KillAnother _asdeath_match_game_mode _asbp_multi_fpsplayer_controller)
  (Utilities|FlowControl|Delay 0.2)
  (Actor|DestroyActor (Pawn|GetControlledPawn))
  (bind _asdeath_match_game_mode_2 (Utilities|Casting|CastToDeathMatchGameMode (Game|GetGameMode)))
  (Default|RequstSpawn _asdeath_match_game_mode_2 self))

(fn ConstructionScript)